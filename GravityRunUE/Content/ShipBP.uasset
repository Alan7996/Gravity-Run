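; Ship actor that moves continuously in the Y-Z plane, steered with the number pad.
; The eight outer keys set a constant-magnitude Speed vector in their compass direction, which persists after release.
; Tick adds Speed to the actor location without sweep or delta-time scaling, so movement depends on frame rate.
; NumPad 5 applies a force opposite to Speed, scaled fivefold, but leaves Speed unchanged.
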(event `Key|NumPadOne`
  (params (Key :type "Key Structure"))
  (:`Pressed`
    (set `self.Speed` (0.0 -7.07 -7.07))))

(event `Key|NumPadTwo`
  (params (Key :type "Key Structure"))
  (:`Pressed`
    (set `self.Speed` (0.0 0.0 -10.0))))

(event `Key|NumPadFive`
  (params (Key :type "Key Structure"))
  (:`Pressed`
    (`PhysicsThreadLibrary.AddForce` (struct) (* (`self.Speed`) (-5.0 -5.0 -5.0)))))

(event `self.ReceiveActorBeginOverlap`
  (params (OtherActor :type "Actor Object Reference")))

(event `Key|NumPadThree`
  (params (Key :type "Key Structure"))
  (:`Pressed`
    (set `self.Speed` (0.0 7.07 -7.07))))

(event `Key|NumPadFour`
  (params (Key :type "Key Structure"))
  (:`Pressed`
    (set `self.Speed` (0.0 -10.0 0.0))))

(event `self.ReceiveTick`
  (params (DeltaSeconds :type "Float (single-precision)"))
  (`self.K2_SetActorLocation` (+ (`self.K2_GetActorLocation`) (`self.Speed`))))

(event `Key|NumPadSix`
  (params (Key :type "Key Structure"))
  (:`Pressed`
    (set `self.Speed` (0.0 10.0 0.0))))

(event `Key|NumPadSeven`
  (params (Key :type "Key Structure"))
  (:`Pressed`
    (set `self.Speed` (0.0 -7.07 7.07))))

(event `Key|NumPadEight`
  (params (Key :type "Key Structure"))
  (:`Pressed`
    (set `self.Speed` (0.0 0.0 10.0))))

(event `Key|NumPadNine`
  (params (Key :type "Key Structure"))
  (:`Pressed`
    (set `self.Speed` (0.0 7.07 7.07))))

(fn `UserConstructionScript`)