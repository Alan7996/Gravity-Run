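; GlobalBP manages laser spawning and the game-over flow for a ship game.
; On BeginPlay a looping timer repeatedly calls SpawnLaser, which spawns a LaserBP at a fixed location with a random roll.
; GameOver prints a death message, shows the mouse cursor, adds the Restart widget to the viewport and calls ShipDead.
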(event `self.ReceiveBeginPlay`
  (`KismetSystemLibrary.K2_SetTimerDelegate` (delegate `SpawnLaserEvent`) 5.0 true))

(event `SpawnLaserEvent`
  (`self.SpawnLaser`))

(event `self.ReceiveTick`
  (params (DeltaSeconds :type "Float (single-precision)")))

(fn `GameOver`
  (`KismetSystemLibrary.PrintString` "You Died!")
  (set `PlayerController.bShowMouseCursor` true (`GameplayStatics.GetPlayerController` 0))
  (bind _returnvalue (`|CreateWidget` "/Game/Restart.Restart_C"))
  (`UserWidget.AddToViewport` _returnvalue 0)
  (`self.ShipDead`))

(fn `SpawnLaser`
  (`|SpawnActorFromClass` "/Game/LaserBP.LaserBP_C" (`KismetMathLibrary.MakeTransform` (2000.0 0.0 0.0) (`KismetMathLibrary.MakeRotator` (`KismetMathLibrary.RandomFloatInRange` 0.0 90.0))) "Undefined" "MultiplyWithRoot" null null))

(fn `UserConstructionScript`)